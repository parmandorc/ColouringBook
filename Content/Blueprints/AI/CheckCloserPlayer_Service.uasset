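; Behavior tree service that keeps an AI targeting the nearer of two local players.
; On each AI tick it compares the controlled pawn's distance to player characters 0 and 1.
; It writes the closer player's controlled pawn to the PlayerKey blackboard entry, choosing player 1 on a tie, with no validity checks.
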(event EventReceiveTickAI
  (params (OwnerController :type AI%20Controller%20Object%20Reference) (ControlledPawn :type Pawn%20Object%20Reference) (DeltaSeconds :type Float%20%28single-precision%29))
  (if (< (Transformation|GetDistanceTo (Game|GetPlayerCharacter 0) ControlledPawn) (Transformation|GetDistanceTo (Game|GetPlayerCharacter 1) ControlledPawn))
    (Class|BTFunctionLibrary|SetBlackboardValueasObject (Variables|Default|GetPlayerKey) (Pawn|GetControlledPawn (Game|GetPlayerController 0)))
    (else
      (Class|BTFunctionLibrary|SetBlackboardValueasObject (Variables|Default|GetPlayerKey) (Pawn|GetControlledPawn (Game|GetPlayerController 1))))))