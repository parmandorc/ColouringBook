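; Behavior tree service that points an AI at the nearer of two players by writing that player's pawn to the PlayerObject blackboard key.
; Each AI tick writes the pawn of the stored Player index, then compares distances from the AI controller to player 0 and player 1 to update the index.
; Because the write precedes the comparison, the blackboard target lags the nearest-player choice by one tick.
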(event EventReceiveTickAI
  (params (OwnerController :type AI%20Controller%20Object%20Reference) (ControlledPawn :type Pawn%20Object%20Reference) (DeltaSeconds :type Float%20%28single-precision%29))
  (bind _returnvalue (AI|GetAIController ControlledPawn))
  (Class|BTFunctionLibrary|SetBlackboardValueasObject (Variables|Default|GetPlayerObject) (Pawn|GetControlledPawn (Game|GetPlayerController (Variables|Default|GetPlayer))))
  (if (< (Transformation|GetDistanceTo _returnvalue (Pawn|GetControlledPawn (Game|GetPlayerController 0))) (Transformation|GetDistanceTo _returnvalue (Pawn|GetControlledPawn (Game|GetPlayerController 1))))
    (Variables|Default|SetPlayer 0)
    (else
      (Variables|Default|SetPlayer 1))))