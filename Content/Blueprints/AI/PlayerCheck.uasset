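; PlayerCheck is an AI Behavior Tree node that keeps the blackboard updated with the player's pawn and position.
; Each tick it reads the pawn controlled by player controller 0 and writes its location and reference to the two player keys.
; When no valid pawn exists, it resets the location to the zero vector, not an unset value, and clears the object key.
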(event EventTick
  (params (OwnerActor :type Actor%20Object%20Reference) (DeltaSeconds :type Float%20%28single-precision%29))
  (bind _returnvalue (Game|GetPlayerController 0))
  (bind _returnvalue_2 (Pawn|GetControlledPawn _returnvalue))
  (if (Utilities|IsValid (Pawn|GetControlledPawn (Game|GetPlayerController 0)))
    (AI|BehaviorTree|SetBlackboardValueasVector (Variables|Default|GetPlayerLocationKey) (Transformation|GetActorLocation _returnvalue_2))
    (Class|BTFunctionLibrary|SetBlackboardValueasObject (Variables|Default|GetPlayerKey) _returnvalue_2)
    (else
      (AI|BehaviorTree|SetBlackboardValueasVector (Variables|Default|GetPlayerLocationKey) "0, 0, 0")
      (Class|BTFunctionLibrary|SetBlackboardValueasObject (Variables|Default|GetPlayerKey)))))