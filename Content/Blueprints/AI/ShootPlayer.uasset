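; ShootPlayer is an AI Behavior Tree task that, judging by its name, is an unfinished attack on the player.
; On execute it caches the pawn as a Character, and its tick holds a timer-gated visibility trace from the pawn to the blackboard player actor.
; Count resets every tick and its increment is unwired, so the trace never fires; no hit handling or finish call exists.
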(event EventReceiveExecuteAI
  (params (OwnerController :type AI%20Controller%20Object%20Reference) (ControlledPawn :type Pawn%20Object%20Reference))
  (bind _ascharacter (Utilities|Casting|CastToCharacter ControlledPawn)))

(event EventReceiveTickAI
  (params (OwnerController :type AI%20Controller%20Object%20Reference) (ControlledPawn :type Pawn%20Object%20Reference) (DeltaSeconds :type Float%20%28single-precision%29))
  (bind _output_get (Variables|Default|SetCount 0.0))
  (if (> _output_get 2.0)
    (Utilities|FlowControl|Sequence
      (:then_0
        (Collision|LineTraceByChannel (Transformation|GetActorLocation (stale EventReceiveExecuteAI ControlledPawn)) (Transformation|GetActorLocation (AI|BehaviorTree|GetBlackboardValueasActor (Variables|Default|GetPlayerKey))) "TraceTypeQuery1" false (Utilities|Array|MakeArray (Components|GetOwner (Variables|/Script/Engine.Character|GetCapsuleComponent (stale EventReceiveExecuteAI _ascharacter)))) "None"))
      (:then_1
        (Variables|Default|SetCount 0.0)))))