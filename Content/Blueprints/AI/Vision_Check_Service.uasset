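; Behavior tree service that gives an AI puppet an angle-based vision check on the player.
; On activation it sets the puppet state key in the Blackboard to a default value.
; Each tick it takes the angle between the pawn's forward vector and the player direction via dot product and inverse cosine.
; Within a 55-degree half-angle it sets the player as target and switches state, with no distance or occlusion test.
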(event EventReceiveTickAI
  (params (OwnerController :type AI%20Controller%20Object%20Reference) (ControlledPawn :type Pawn%20Object%20Reference) (DeltaSeconds :type Float%20%28single-precision%29))
  (if (< (Class|KismetMathLibrary|DegAcos (Math|Vector|DotProduct (Math|Vector|Normalize (- (Transformation|GetActorLocation (AI|BehaviorTree|GetBlackboardValueasActor (Variables|Default|GetPlayer_Key_BP))) (Transformation|GetActorLocation ControlledPawn))) (Transformation|GetActorForwardVector ControlledPawn))) 55.0) ; Can the AI see the player?
    (Class|BTFunctionLibrary|SetBlackboardValueasObject (Variables|Default|GetTargetActor) (AI|BehaviorTree|GetBlackboardValueasActor (Variables|Default|GetPlayer_Key_BP)))
    (Class|BTFunctionLibrary|SetBlackboardValueasEnum (Variables|Default|GetState_Key) (Utilities|Enum|LiteralenumPuppet_State "NewEnumerator0"))))

(event EventReceiveActivationAI
  (params (OwnerController :type AI%20Controller%20Object%20Reference) (ControlledPawn :type Pawn%20Object%20Reference))
  (Class|BTFunctionLibrary|SetBlackboardValueasEnum (Variables|Default|GetState_Key) (Utilities|Enum|LiteralenumPuppet_State "NewEnumerator1")))